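; Key spawner actor that pops out a single BP_Key when the player presses while standing near it.
; Sphere overlap events track whether the player pawn is in range.
; Tick polls BP_Player's IsPressed flag, and a DoOnce limits spawning to one key.
; The key spawns at SpawnPoint's location and rotation, then gets a fixed velocity-change impulse that tosses it up and along world X.
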(event OnComponentBeginOverlap(Sphere)
  (params (OverlappedComponent :type Primitive%20Component%20Object%20Reference) (OtherActor :type Actor%20Object%20Reference) (OtherComp :type Primitive%20Component%20Object%20Reference) (OtherBodyIndex :type Integer) (bFromSweep :type Boolean) (SweepResult :type Hit%20Result%20Structure%20%28by%20ref%29))
  ;[1 1 1] Set IsOverlapping
  (if (== OtherActor (Game|Player|GetPlayerPawn 0))
    (Variables|Default|SetisOverlapping true)))

(event OnComponentEndOverlap(Sphere)
  (params (OverlappedComponent :type Primitive%20Component%20Object%20Reference) (OtherActor :type Actor%20Object%20Reference) (OtherComp :type Primitive%20Component%20Object%20Reference) (OtherBodyIndex :type Integer))
  ;[1 1 1] Set IsOverlapping
  (if (== OtherActor (Game|Player|GetPlayerPawn 0))
    (Variables|Default|SetisOverlapping false)))

(event EventTick
  (params (DeltaSeconds :type Float%20%28single-precision%29))
  (bind _spawnpoint (Variables|Default|GetSpawnPoint))
  (bind _returnvalue (Transformation|GetWorldTransform _spawnpoint))
  (bind (_location _rotation) (Math|Transform|BreakTransform _returnvalue))
  ;[1 1 1] Spawn Key
  (bind _asbp_player (Utilities|Casting|CastToBP_Player (Game|Player|GetPlayerPawn 0)))
  (if (Variables|/Game/Blueprints/BP_Player.BP_Player_C|GetIsPressed _asbp_player)
    (if (Variables|Default|GetisOverlapping)
      (Utilities|FlowControl|DoOnce false
        (:Completed
          (bind _returnvalue_2 (Game|SpawnActorfromClass "/Game/Blueprints/BP_Key.BP_Key_C" (Math|Transform|MakeTransform _location _rotation "1.000000,1.000000,1.000000") "Undefined" 0 0))
          (Physics|AddImpulse (Variables|/Game/Blueprints/BP_Key.BP_Key_C|GetStaticMesh _returnvalue_2) "150.000000, 0,500.000000" "None" true))))))

(fn ConstructionScript)