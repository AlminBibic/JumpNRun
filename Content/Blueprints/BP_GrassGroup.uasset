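; BP_GrassGroup is a cluster of static meshes, named as grass, that orients itself to the surface of a planet.
; Its construction script picks a BP_Planet by the Planet index from all such actors.
; It rotates the actor so Z points away from the planet's center, using the main mesh's forward vector for X.
; It then pushes LightFactor into the Lightfactor material parameter on all ten meshes.
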(event EventBeginPlay)

(event Collision|EventActorBeginOverlap
  (params (OtherActor :type Actor%20Object%20Reference)))

(event EventTick
  (params (DeltaSeconds :type Float%20%28single-precision%29)))

(fn ConstructionScript
  (Utilities|FlowControl|Sequence
    (:then_0
      (bind _outactors (Actor|GetAllActorsOfClass "/Game/Blueprints/BP_Planet.BP_Planet_C"))
      (Variables|Default|SetPlanetBP (Utilities|Array|Get(acopy) _outactors (Variables|Default|GetPlanet))))
    (:then_1
      (Transformation|SetActorRotation (Math|Rotator|MakeRotfromZX (Math|Vector|GetForwardVector (Math|Rotator|FindLookatRotation (Transformation|GetActorLocation (Variables|Default|GetPlanetBP)) (Transformation|GetActorLocation))) (Math|Vector|GetForwardVector (Variables|Default|GetStaticMesh)))))
    (:then_2
      (Rendering|Material|SetScalarParameterValueonMaterials (Variables|Default|GetStaticMesh) "Lightfactor" (Variables|Default|GetLightFactor)))))