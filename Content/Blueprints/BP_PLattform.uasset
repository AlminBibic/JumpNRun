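; Platform that plays a timed ride sequence once the player presses inside its trigger box while holding three keys.
; Tick polls that condition, then eases the base toward a target point with VInterpTo.
; On start, the camera blends to the platform and its stand-in skeletal mesh replaces the hidden player mesh.
; After a fixed delay, the pawn teleports to the teleport point, the camera blends back and mesh visibility is restored.
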(event OnComponentBeginOverlap(Box)
  (params (OverlappedComponent :type Primitive%20Component%20Object%20Reference) (OtherActor :type Actor%20Object%20Reference) (OtherComp :type Primitive%20Component%20Object%20Reference) (OtherBodyIndex :type Integer) (bFromSweep :type Boolean) (SweepResult :type Hit%20Result%20Structure%20%28by%20ref%29))
  ;[1 1 1] Set is Overlapping
  (if (== OtherActor (Game|Player|GetPlayerPawn 0))
    (Variables|Default|SetIsOverlapping true)))

(event OnComponentEndOverlap(Box)
  (params (OverlappedComponent :type Primitive%20Component%20Object%20Reference) (OtherActor :type Actor%20Object%20Reference) (OtherComp :type Primitive%20Component%20Object%20Reference) (OtherBodyIndex :type Integer))
  ;[1 1 1] Set is Overlapping
  (if (== OtherActor (Game|Player|GetPlayerPawn 0))
    (Variables|Default|SetIsOverlapping false)))

(event Custom|MovePlattform
  (bind _base (Variables|Default|GetBase))
  ;[1 1 1] Move Plattform
  (Transformation|SetWorldLocation _base (Math|Interpolation|VInterpTo (Transformation|GetWorldLocation _base) (Transformation|GetWorldLocation (Variables|/Script/Engine.TargetPoint|GetSpriteComponent (Variables|Default|GetTargetPoit))) (Utilities|Time|GetWorldDeltaSeconds) 0.1) false false)
  (Utilities|FlowControl|DoOnce false
    (:Completed
      (Development|SetHiddeninGame (Variables|Default|GetSkeletalMesh) false false)
      (Game|Player|SetViewTargetwithBlend (Game|GetPlayerController 0) self 2.0 "VTBlend_Linear" 0.0 false)
      (bind _asbp_player (Utilities|Casting|CastToBP_Player (Game|Player|GetPlayerPawn 0)))
      (Development|SetHiddeninGame (Variables|/Game/Blueprints/BP_Player.BP_Player_C|GetSkeletalMesh _asbp_player) true false)
      (Utilities|FlowControl|Delay 28.0)
      (Transformation|SetWorldLocation (Variables|/Script/Engine.Actor|GetRootComponent (Game|Player|GetPlayerPawn 0)) (Transformation|GetWorldLocation (Variables|/Script/Engine.Actor|GetRootComponent (Variables|Default|GetTeleportPoint))) false true)
      (Game|Player|SetViewTargetwithBlend (Game|GetPlayerController 0) (Game|Player|GetPlayerPawn 0) 2.0 "VTBlend_Linear" 0.0 false))))

(event EventTick
  (params (DeltaSeconds :type Float%20%28single-precision%29))
  (Utilities|FlowControl|Sequence
    (:then_0
      (if (Variables|Default|GetStart)
        (CallFunction|MovePlattform)))
    (:then_1
      (if (Variables|Default|GetIsOverlapping)
        (bind _asbp_player (Utilities|Casting|CastToBP_Player (Game|Player|GetPlayerPawn 0)))
        (if (Variables|/Game/Blueprints/BP_Player.BP_Player_C|GetIsPressed _asbp_player)
          (if (== (Variables|/Game/Blueprints/BP_Player.BP_Player_C|GetKeys _asbp_player) 3)
            (Variables|Default|SetStart true)))))
    (:then_2
      (if (Variables|Default|GetStart)
        (Utilities|FlowControl|Delay 28.0)
        (Utilities|FlowControl|DoOnce false
          (:Completed
            (bind _asbp_player_2 (Utilities|Casting|CastToBP_Player (Game|Player|GetPlayerPawn 0)))
            (Development|SetHiddeninGame (Variables|/Game/Blueprints/BP_Player.BP_Player_C|GetSkeletalMesh _asbp_player_2) false false)
            (Development|SetHiddeninGame (Variables|Default|GetSkeletalMesh) true false)))))))

(event EventBeginPlay
  (Development|SetHiddeninGame (Variables|Default|GetSkeletalMesh) true false))

(fn ConstructionScript)