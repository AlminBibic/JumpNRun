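; BP_Dummy is a self-moving physics actor that travels around a BP_Planet and knocks the player on contact.
; Each tick it aligns its up axis away from the planet center, adds velocity toward the planet as custom gravity, and adds forward velocity.
; Two child meshes spin continuously at different rates.
; When its capsule overlaps the player pawn, it adds KnockBackPower-scaled velocity along the player mesh's forward vector.
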(event OnComponentBeginOverlap(Capsule)
  (params (OverlappedComponent :type Primitive%20Component%20Object%20Reference) (OtherActor :type Actor%20Object%20Reference) (OtherComp :type Primitive%20Component%20Object%20Reference) (OtherBodyIndex :type Integer) (bFromSweep :type Boolean) (SweepResult :type Hit%20Result%20Structure%20%28by%20ref%29))
  (if (== OtherActor (Game|Player|GetPlayerPawn 0))
    (bind _asbp_player (Utilities|Casting|CastToBP_Player (Game|Player|GetPlayerPawn 0)))
    (Physics|SetPhysicsLinearVelocity (Variables|/Game/Blueprints/BP_Player.BP_Player_C|GetStaticMesh _asbp_player) (* (Math|Vector|GetForwardVector (Variables|/Game/Blueprints/BP_Player.BP_Player_C|GetStaticMesh _asbp_player)) (Variables|Default|GetKockBackPower)) true "None")))

(event Custom|Move
  ;[1 1 1] Move event
  (Physics|SetPhysicsLinearVelocity (Variables|Default|GetStaticMesh) (* (Math|Vector|GetForwardVector (Variables|Default|GetStaticMesh)) (Variables|Default|GetAcceleration)) true "None"))

(event Custom|Spin
  (bind _staticmesh1 (Variables|Default|GetStaticMesh1))
  (bind _staticmesh2 (Variables|Default|GetStaticMesh2))
  (bind _relativerotation (Variables|/Script/Engine.SceneComponent|GetRelativeRotation _staticmesh2))
  (bind _relativerotation_2 (Variables|/Script/Engine.SceneComponent|GetRelativeRotation _staticmesh1))
  ;[1 1 1] Spin
  (Transformation|SetRelativeRotation _staticmesh1 (Math|Rotator|MakeRotator (.roll _relativerotation_2) (.pitch _relativerotation_2) (+ (.yaw _relativerotation_2) 6.0)) false false)
  (Transformation|SetRelativeRotation (Variables|Default|GetStaticMesh2) (Math|Rotator|MakeRotator (.roll _relativerotation) (.pitch _relativerotation) (+ (.yaw _relativerotation) 1e+01)) false false))

(event EventTick
  (params (DeltaSeconds :type Float%20%28single-precision%29))
  (bind _returnvalue (Transformation|GetActorLocation))
  (bind _planetbp (Variables|Default|GetPlanetBP))
  (bind _returnvalue_2 (Transformation|GetActorLocation _planetbp))
  (bind _returnvalue_3 (Math|Rotator|FindLookatRotation _returnvalue_2 _returnvalue))
  (bind _returnvalue_4 (Math|Vector|GetForwardVector _returnvalue_3))
  ;[1 1 1] Set Rotation and Move
  (Transformation|SetActorRotation (Math|Rotator|MakeRotfromZX _returnvalue_4 (Math|Vector|GetForwardVector (Variables|Default|GetStaticMesh))))
  (Physics|SetPhysicsLinearVelocity (Variables|Default|GetStaticMesh) (* (* _returnvalue_4 -1) (Variables|Default|GetAcceleration)) true "None")
  (CallFunction|Move)
  (CallFunction|Spin))

(event EventBeginPlay
  ;[1 1 1] Get Planet
  (bind _outactors (Actor|GetAllActorsOfClass "/Game/Blueprints/BP_Planet.BP_Planet_C"))
  (Variables|Default|SetPlanetBP (Utilities|Array|Get(acopy) _outactors (Variables|Default|GetPlanet))))

(fn ConstructionScript)