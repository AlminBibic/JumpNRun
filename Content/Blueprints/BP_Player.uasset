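; BP_Player is a physics-driven player pawn that walks on spherical planets, with jump, roll, water-jet attack and an idle sleep flag.
; Tick picks the nearest planet surface, pulls the body toward its center and eases the actor upright to it.
; Firing line-traces for HIT-tagged components and damages the first BP_Tentacle found.
; At zero health it swaps to a simulated Hippo ragdoll, shows a fade and opens Level_Test.
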(event OnComponentHit(StaticMesh)
  (params (HitComponent :type Primitive%20Component%20Object%20Reference) (OtherActor :type Actor%20Object%20Reference) (OtherComp :type Primitive%20Component%20Object%20Reference) (NormalImpulse :type Vector :default "0, 0, 0") (Hit :type Hit%20Result%20Structure%20%28by%20ref%29))
  (bind _staticmesh (Variables|Default|GetStaticMesh))
  ;[1 1 1] Input
  (Variables|Default|SetIsFalling false)
  (Utilities|FlowControl|DoOnce false) ; enters at Reset
)

(event Custom|CheckIsFiring
  (bind _muzzle (Variables|Default|GetMuzzle))
  (bind _returnvalue (Transformation|GetWorldLocation _muzzle))
  ;[1 1 1] Input
  (if (Variables|Default|GetIsFiring)
    (Development|SetHiddeninGame (Variables|Default|GetWaterFountain) false false)
    (Utilities|FlowControl|Delay 0.3)
    (bind _outhit (Collision|LineTraceByChannel _returnvalue (+ _returnvalue (* (Math|Vector|GetRightVector (Variables|Default|GetSkeletalMesh)) (Variables|Default|GetDistance))) "TraceTypeQuery1" false 0 "ForDuration" true "(R=1.000000,G=0.000000,B=0.000000,A=1.000000)" "(R=0.000000,G=1.000000,B=0.000000,A=1.000000)" 2.0))
    (Utilities|IsValid (.HitActor (Collision|BreakHitResult _outhit))
      (:Is%20Valid
        (if (Components|ComponentHasTag (.HitComponent (Collision|BreakHitResult _outhit)) "HIT")
          (bind _outactors (Actor|GetAllActorsOfClass "/Game/Blueprints/BP_Tentacle.BP_Tentacle_C"))
          (bind _output_get (Variables|Default|SetTentacleRef (Utilities|Array|Get(acopy) _outactors)))
          (bind _asbp_tentacle (Utilities|Casting|CastToBP_Tentacle _output_get))
          (Variables|/Game/Blueprints/BP_Tentacle.BP_Tentacle_C|SetHealthPoints _asbp_tentacle (- (Variables|/Game/Blueprints/BP_Tentacle.BP_Tentacle_C|GetHealthPoints _asbp_tentacle) 1))
          (Effects|SpawnEmitteratLocation "/Game/Particles/P_Blood.P_Blood" (.Location (Collision|BreakHitResult _outhit)) "0, 0, 0" "0.250000,0.250000,0.250000"))))))

(event Custom|RagDolldeath
  ;[1 1 1] Check if Dead and then apply Ragdoll Death
  (if (<= (Variables|Default|GetHealthPoints) 0)
    (Development|SetHiddeninGame (Variables|Default|GetSkeletalMesh) true false)
    (Development|SetHiddeninGame (Variables|Default|GetHippo) false false)
    (Physics|SetSimulatePhysics (Variables|Default|GetHippo) true)
    (Physics|AddImpulse (Variables|Default|GetHippo) (* (Math|Vector|GetForwardVector (Variables|Default|GetStaticMesh)) -1.0) "None" true)
    (bind _returnvalue (UserInterface|CreateWidget "/Game/Blueprints/WBP_Fade.WBP_Fade_C"))
    (UserInterface|Viewport|AddtoViewport _returnvalue 0)
    (Utilities|FlowControl|Delay 4.3)
    (Game|OpenLevel(byName) "Level_Test")))

(event Custom|Sleeping
  ;[1 1 1] Sleep
  (Utilities|FlowControl|Delay 9e+01)
  (Variables|Default|Setsleep true))

(event EventTick
  (params (DeltaSeconds :type Float%20%28single-precision%29))
  (bind _returnvalue (Transformation|GetActorLocation))
  (bind _planetbp (Variables|Default|GetPlanetBP))
  (bind _planetbp_2 (Variables|Default|GetPlanetBP))
  (bind _returnvalue_2 (Transformation|GetActorLocation _planetbp_2))
  (bind _returnvalue_3 (Math|Rotator|FindLookatRotation _returnvalue_2 _returnvalue))
  (bind _returnvalue_4 (Math|Vector|GetForwardVector _returnvalue_3))
  ;[1 1 1] Set Rotation and Current Planet
  (Transformation|SetActorRotation (Math|Interpolation|Ease "Linear" (Math|Float|Clamp(Float) (/ 1e+01 (- (Math|Vector|VectorLength (- (Transformation|GetActorLocation) (Transformation|GetActorLocation _planetbp))) (* (.X (Math|Vector|BreakVector (Transformation|GetWorldScale (Variables|/Game/Blueprints/BP_Planet.BP_Planet_C|GetStaticMesh _planetbp)))) 5e+01))) 0.01) (Transformation|GetActorRotation) (Math|Rotator|MakeRotfromZX _returnvalue_4 (Math|Vector|GetForwardVector (Variables|Default|GetStaticMesh))) true))
  (Physics|SetPhysicsLinearVelocity (Variables|Default|GetStaticMesh) (* (* _returnvalue_4 -1) (Variables|Default|GetAcceleration)) true "None")
  (CallFunction|SetPlanet)
  (CallFunction|CheckIsFiring)
  (CallFunction|Sleeping)
  (CallFunction|RagDolldeath))

(event EventBeginPlay
  (bind _outactors (Actor|GetAllActorsOfClass "/Game/Blueprints/BP_Planet.BP_Planet_C"))
  (Variables|Default|SetPlanets _outactors)
  (Variables|Default|SetPlanetBP (Utilities|Array|Get(acopy) _outactors))
  (Development|SetHiddeninGame (Variables|Default|GetWaterFountain) true false))

(event Input|ActionEvents|InputActionJump
  (params (Key :type Key%20Structure))
  (bind _staticmesh (Variables|Default|GetStaticMesh))
  ;[1 1 1] Input
  (:Pressed
    (Variables|Default|Setsleep false)
    (Utilities|FlowControl|DoOnce false
      (:Completed
        (Physics|SetPhysicsLinearVelocity _staticmesh (* (Math|Vector|GetUpVector _staticmesh) 1.5e+03) true "None")
        (Variables|Default|SetIsFalling true)))))

(event Input|ActionEvents|InputActionInteract
  (params (Key :type Key%20Structure))
  ;[1 1 1] Set IsPressed
  (:Pressed
    (bind _output_get (Variables|Default|SetIsPressed true))
    (Development|PrintString (Utilities|String|ToString(Boolean) _output_get)))
  (:Released
    (bind _output_get_2 (Variables|Default|SetIsPressed false))
    (Development|PrintString (Utilities|String|ToString(Boolean) _output_get_2))))

(event Input|ActionEvents|InputActionRoll
  (params (Key :type Key%20Structure))
  ;[1 1 1] Input
  (:Pressed
    (Variables|Default|Setsleep false)
    (if (not (Variables|Default|GetIsRolling))
      (Physics|AddImpulse (Variables|Default|GetStaticMesh) (* (Math|Vector|GetForwardVector (Variables|Default|GetArrow)) 1e+03) "None" true)
      (Variables|Default|SetIsRolling true)
      (Utilities|FlowControl|Delay 0.5)
      (Variables|Default|SetIsRolling false))))

(event Input|ActionEvents|InputActionFire
  (params (Key :type Key%20Structure))
  ;[1 1 1] Input
  (:Pressed
    (Variables|Default|SetIsFiring true)
    (Variables|Default|Setsleep false))
  (:Released
    (Variables|Default|SetIsFiring false)
    (Development|SetHiddeninGame (Variables|Default|GetWaterFountain) true false)))

(event Input|AxisEvents|InputAxisMoveForward
  (params (AxisValue :type Float%20%28single-precision%29))
  ;[1 1 1] Input
  (Physics|SetPhysicsLinearVelocity (Variables|Default|GetStaticMesh) (* (* (Math|Vector|GetForwardVector (Variables|Default|GetStaticMesh)) AxisValue) (Variables|Default|GetAcceleration)) true "None")
  (Utilities|FlowControl|Sequence
    (:then_0
      (if (> AxisValue 0.0)
        (Transformation|SetRelativeRotation (Variables|Default|GetSkeletalMesh) "0,-90.000000, 0" false false)
        (Variables|Default|Setsleep false)))
    (:then_1
      (if (< AxisValue 0.0)
        (Transformation|SetRelativeRotation (Variables|Default|GetSkeletalMesh) "0,90.000000, 0" false false)
        (Variables|Default|Setsleep false)))))

(event Input|AxisEvents|InputAxisMoveRight
  (params (AxisValue :type Float%20%28single-precision%29))
  ;[1 1 1] Input
  (Physics|SetPhysicsLinearVelocity (Variables|Default|GetStaticMesh) (* (* (Math|Vector|GetRightVector (Variables|Default|GetStaticMesh)) AxisValue) (Variables|Default|GetAcceleration)) true "None")
  (Utilities|FlowControl|Sequence
    (:then_0
      (if (> AxisValue 0.0)
        (Transformation|SetRelativeRotation (Variables|Default|GetSkeletalMesh) "0, 0, 0" false false)
        (Variables|Default|Setsleep false)))
    (:then_1
      (if (< AxisValue 0.0)
        (Transformation|SetRelativeRotation (Variables|Default|GetSkeletalMesh) "0,-180.000000, 0" false false)
        (Variables|Default|Setsleep false)))))

(event Input|AxisEvents|InputAxisLookUp
  (params (AxisValue :type Float%20%28single-precision%29))
  ;[1 1 1] Input
  (Transformation|AddLocalRotation (Variables|Default|GetSpringArm) (Math|Rotator|MakeRotator 0.0 AxisValue 0.0) false false))

(event Input|AxisEvents|InputAxisTurn
  (params (AxisValue :type Float%20%28single-precision%29))
  ;[1 1 1] Input
  (Transformation|AddLocalRotation (Variables|Default|GetStaticMesh) (Math|Rotator|MakeRotator 0.0 0.0 AxisValue) false false))

(event Input|KeyboardEvents|I
  (params (Key :type Key%20Structure))
  ;[1 1 1] Input
  (:Pressed
    (Variables|Default|SetVic true)
    (Variables|Default|Setsleep false))
  (:Released
    (Variables|Default|SetVic false)))

(fn ConstructionScript)

(fn SetPlanet
  (for _array_element (Variables|Default|GetPlanets)
    (if (< (- (Math|Vector|VectorLength (- (Transformation|GetActorLocation _array_element) (Transformation|GetActorLocation))) (* 5e+01 (.x (Transformation|GetActorScale3D _array_element)))) (- (Math|Vector|VectorLength (- (Transformation|GetActorLocation (Variables|Default|GetPlanetBP)) (Transformation|GetActorLocation))) (* 5e+01 (.x (Transformation|GetActorScale3D (Variables|Default|GetPlanetBP))))))
      (Variables|Default|SetPlanetBP _array_element))))