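; Rotating fire hazard with up to four flames that knocks back and damages the player.
; Tick yaws FireHolder each frame, using latent Delays to alternate spinning with timed pauses.
; Four capsule overlaps share one hit response: add velocity along the player mesh's forward vector and subtract one health point.
; Tick also checks per-flame Off flags, destroying the matching particle and capsule to disable that flame.
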(event OnComponentBeginOverlap(Capsule)
  (params (OverlappedComponent :type Primitive%20Component%20Object%20Reference) (OtherActor :type Actor%20Object%20Reference) (OtherComp :type Primitive%20Component%20Object%20Reference) (OtherBodyIndex :type Integer) (bFromSweep :type Boolean) (SweepResult :type Hit%20Result%20Structure%20%28by%20ref%29))
  ;[1 1 1] Collision With Fire
  (if (== OtherActor (Game|Player|GetPlayerPawn 0))
    (Development|PrintString "Your are hit by Fire")
    (bind _asbp_player (Utilities|Casting|CastToBP_Player (Game|Player|GetPlayerPawn 0)))
    (Physics|SetPhysicsLinearVelocity (Variables|/Game/Blueprints/BP_Player.BP_Player_C|GetStaticMesh _asbp_player) (* (Math|Vector|GetForwardVector (Variables|/Game/Blueprints/BP_Player.BP_Player_C|GetStaticMesh _asbp_player)) (Variables|Default|GetKnockBackPower)) true "None")
    (Variables|/Game/Blueprints/BP_Player.BP_Player_C|SetHealthPoints _asbp_player (- (Variables|/Game/Blueprints/BP_Player.BP_Player_C|GetHealthPoints _asbp_player) 1))))

(event OnComponentBeginOverlap(Capsule1)
  (params (OverlappedComponent :type Primitive%20Component%20Object%20Reference) (OtherActor :type Actor%20Object%20Reference) (OtherComp :type Primitive%20Component%20Object%20Reference) (OtherBodyIndex :type Integer) (bFromSweep :type Boolean) (SweepResult :type Hit%20Result%20Structure%20%28by%20ref%29))
  ;[1 1 1] Collision With Fire
  (if (== OtherActor (Game|Player|GetPlayerPawn 0))
    (Development|PrintString "Your are hit by Fire")
    (bind _asbp_player (Utilities|Casting|CastToBP_Player (Game|Player|GetPlayerPawn 0)))
    (Physics|SetPhysicsLinearVelocity (Variables|/Game/Blueprints/BP_Player.BP_Player_C|GetStaticMesh _asbp_player) (* (Math|Vector|GetForwardVector (Variables|/Game/Blueprints/BP_Player.BP_Player_C|GetStaticMesh _asbp_player)) (Variables|Default|GetKnockBackPower)) true "None")
    (Variables|/Game/Blueprints/BP_Player.BP_Player_C|SetHealthPoints _asbp_player (- (Variables|/Game/Blueprints/BP_Player.BP_Player_C|GetHealthPoints _asbp_player) 1))))

(event OnComponentBeginOverlap(Capsule2)
  (params (OverlappedComponent :type Primitive%20Component%20Object%20Reference) (OtherActor :type Actor%20Object%20Reference) (OtherComp :type Primitive%20Component%20Object%20Reference) (OtherBodyIndex :type Integer) (bFromSweep :type Boolean) (SweepResult :type Hit%20Result%20Structure%20%28by%20ref%29))
  ;[1 1 1] Collision With Fire
  (if (== OtherActor (Game|Player|GetPlayerPawn 0))
    (Development|PrintString "Your are hit by Fire")
    (bind _asbp_player (Utilities|Casting|CastToBP_Player (Game|Player|GetPlayerPawn 0)))
    (Physics|SetPhysicsLinearVelocity (Variables|/Game/Blueprints/BP_Player.BP_Player_C|GetStaticMesh _asbp_player) (* (Math|Vector|GetForwardVector (Variables|/Game/Blueprints/BP_Player.BP_Player_C|GetStaticMesh _asbp_player)) (Variables|Default|GetKnockBackPower)) true "None")
    (Variables|/Game/Blueprints/BP_Player.BP_Player_C|SetHealthPoints _asbp_player (- (Variables|/Game/Blueprints/BP_Player.BP_Player_C|GetHealthPoints _asbp_player) 1))))

(event OnComponentBeginOverlap(Capsule3)
  (params (OverlappedComponent :type Primitive%20Component%20Object%20Reference) (OtherActor :type Actor%20Object%20Reference) (OtherComp :type Primitive%20Component%20Object%20Reference) (OtherBodyIndex :type Integer) (bFromSweep :type Boolean) (SweepResult :type Hit%20Result%20Structure%20%28by%20ref%29))
  ;[1 1 1] Collision With Fire
  (if (== OtherActor (Game|Player|GetPlayerPawn 0))
    (Development|PrintString "Your are hit by Fire")
    (bind _asbp_player (Utilities|Casting|CastToBP_Player (Game|Player|GetPlayerPawn 0)))
    (Physics|SetPhysicsLinearVelocity (Variables|/Game/Blueprints/BP_Player.BP_Player_C|GetStaticMesh _asbp_player) (* (Math|Vector|GetForwardVector (Variables|/Game/Blueprints/BP_Player.BP_Player_C|GetStaticMesh _asbp_player)) (Variables|Default|GetKnockBackPower)) true "None")
    (Variables|/Game/Blueprints/BP_Player.BP_Player_C|SetHealthPoints _asbp_player (- (Variables|/Game/Blueprints/BP_Player.BP_Player_C|GetHealthPoints _asbp_player) 1))))

(event Custom|Spin
  (bind _fireholder (Variables|Default|GetFireHolder))
  (bind _fireholder_2 (Variables|Default|GetFireHolder))
  (bind _relativerotation (Variables|/Script/Engine.SceneComponent|GetRelativeRotation _fireholder))
  ;[1 1 1] Spin and Stop
  (if (not (Variables|Default|GetIsStoped))
    (Transformation|SetRelativeRotation (Variables|Default|GetFireHolder) (Math|Rotator|MakeRotator (.roll _relativerotation) (.pitch _relativerotation) (+ (.yaw _relativerotation) 1.0)) false false)
    (Utilities|FlowControl|Delay 1e+01)
    (Variables|Default|SetIsStoped true)
    (Transformation|SetRelativeRotation _fireholder_2 (Variables|/Script/Engine.SceneComponent|GetRelativeRotation _fireholder_2) false false)
    (Utilities|FlowControl|Delay 5.0)
    (Variables|Default|SetIsStoped false)))

(event Custom|CheckFire
  (bind _particlesystem (Variables|Default|GetParticleSystem))
  (bind _particlesystem1 (Variables|Default|GetParticleSystem1))
  (bind _particlesystem2 (Variables|Default|GetParticleSystem2))
  (bind _particlesystem3 (Variables|Default|GetParticleSystem3))
  ;[1 1 1] Check Fire
  (Utilities|FlowControl|Sequence
    (:then_0
      (if (Variables|Default|GetFireOneOff)
        (Utilities|IsValid _particlesystem
          (:Is%20Valid
            (Utilities|IsValid (Variables|Default|GetCapsule)
              (:Is%20Valid
                (Components|DestroyComponent _particlesystem)))))))
    (:then_1
      (if (Variables|Default|GetFireTwoOff)
        (Utilities|IsValid _particlesystem1
          (:Is%20Valid
            (Utilities|IsValid (Variables|Default|GetCapsule1)
              (:Is%20Valid
                (Components|DestroyComponent _particlesystem1)))))))
    (:then_2
      (if (Variables|Default|GetFireThreeOff)
        (Utilities|IsValid _particlesystem2
          (:Is%20Valid
            (Utilities|IsValid (Variables|Default|GetCapsule2)
              (:Is%20Valid
                (Components|DestroyComponent _particlesystem2)))))))
    (:then_3
      (if (Variables|Default|GetFireFourOff)
        (Utilities|IsValid _particlesystem3
          (:Is%20Valid
            (Utilities|IsValid (Variables|Default|GetCapsule3)
              (:Is%20Valid
                (Components|DestroyComponent _particlesystem3)))))))))

(event EventTick
  (params (DeltaSeconds :type Float%20%28single-precision%29))
  (CallFunction|Spin)
  (CallFunction|CheckFire))

(fn ConstructionScript)