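; BP_WoodStump is the level's win trigger, completed when an overlapping player presses interact while holding exactly three keys.
; Its box overlap toggles a sprite and text prompt, while Tick polls the player's input and key count to set Win.
; Once won, Tick repeatedly lowers a material Alpha on two meshes.
; A DoOnce clears keys, blends to a camera actor, swaps skeletal mesh visibility and disables input, before a delayed camera fade.
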(event OnComponentBeginOverlap(Box)
  (params (OverlappedComponent :type Primitive%20Component%20Object%20Reference) (OtherActor :type Actor%20Object%20Reference) (OtherComp :type Primitive%20Component%20Object%20Reference) (OtherBodyIndex :type Integer) (bFromSweep :type Boolean) (SweepResult :type Hit%20Result%20Structure%20%28by%20ref%29))
  ;[1 1 1] Set IsOverlapping
  (if (== OtherActor (Game|Player|GetPlayerPawn 0))
    (Variables|Default|SetIsOverlapping true)
    (Development|SetHiddeninGame (Variables|Default|GetPaperSprite) false false)))

(event OnComponentEndOverlap(Box)
  (params (OverlappedComponent :type Primitive%20Component%20Object%20Reference) (OtherActor :type Actor%20Object%20Reference) (OtherComp :type Primitive%20Component%20Object%20Reference) (OtherBodyIndex :type Integer))
  ;[1 1 1] Set IsOverlapping
  (if (== OtherActor (Game|Player|GetPlayerPawn 0))
    (Variables|Default|SetIsOverlapping false)
    (Development|SetHiddeninGame (Variables|Default|GetPaperSprite) true false)))

(event Custom|Victory
  ;[1 1 1] Victory Event
  (bind _output_get (Variables|Default|SetAlpha (Math|Float|Clamp(Float) (- (Variables|Default|GetAlpha) 0.001))))
  (Rendering|Material|SetScalarParameterValueonMaterials (Variables|Default|GetStaticMesh1) "Alpha" _output_get)
  (Utilities|FlowControl|DoOnce false
    (:Completed
      (bind _asbp_player (Utilities|Casting|CastToBP_Player (Game|Player|GetPlayerPawn 0)))
      (Variables|/Game/Blueprints/BP_Player.BP_Player_C|SetKeys _asbp_player 0)
      (Game|Player|SetViewTargetwithBlend (Game|GetPlayerController 0) (Variables|Default|GetCameraActor) 2.0 "VTBlend_Linear" 0.0 false)
      (Utilities|FlowControl|Delay 3.0)
      (Development|SetHiddeninGame (Variables|Default|GetSkeletalMesh) false false)
      (Development|SetHiddeninGame (Variables|/Game/Blueprints/BP_Player.BP_Player_C|GetSkeletalMesh _asbp_player) true false)
      (Input|DisableInput (Game|GetPlayerController 0) 0))))

(event EventBeginPlay)

(event Collision|EventActorBeginOverlap
  (params (OtherActor :type Actor%20Object%20Reference)))

(event EventTick
  (params (DeltaSeconds :type Float%20%28single-precision%29))
  (Utilities|FlowControl|Sequence
    (:then_0
      (if (Variables|Default|GetWin)
        (CallFunction|Victory)
        (Utilities|FlowControl|Delay 1e+01)
        (CameraFades|StartCameraFade :self (Game|GetPlayerCameraManager 0) :ToAlpha 1.0 :Duration 2.0 :bHoldWhenFinished true)))
    (:then_1
      (if (Variables|Default|GetIsOverlapping)
        (bind _asbp_player (Utilities|Casting|CastToBP_Player (Game|Player|GetPlayerPawn 0)))
        (if (Variables|/Game/Blueprints/BP_Player.BP_Player_C|GetIsPressed _asbp_player)
          (if (== (Variables|/Game/Blueprints/BP_Player.BP_Player_C|GetKeys _asbp_player) 3)
            (Variables|Default|SetWin true)))))))

(fn ConstructionScript)