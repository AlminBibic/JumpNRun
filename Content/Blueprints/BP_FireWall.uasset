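; BP_FireWall is a hazard that damages and launches the player on contact.
; When the player pawn begins overlapping its box, a knockback event casts that pawn to BP_Player.
; It adds physics velocity to the player's static mesh along the mesh's forward vector, scaled by KnockBackPower, and subtracts one health point.
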(event OnComponentBeginOverlap(Box)
  (params (OverlappedComponent :type Primitive%20Component%20Object%20Reference) (OtherActor :type Actor%20Object%20Reference) (OtherComp :type Primitive%20Component%20Object%20Reference) (OtherBodyIndex :type Integer) (bFromSweep :type Boolean) (SweepResult :type Hit%20Result%20Structure%20%28by%20ref%29))
  (if (== OtherActor (Game|Player|GetPlayerPawn 0))
    (CallFunction|KnockBack)))

(event Custom|KnockBack
  ;[1 1 1] Knockback
  (bind _asbp_player (Utilities|Casting|CastToBP_Player (Game|Player|GetPlayerPawn 0)))
  (Physics|SetPhysicsLinearVelocity (Variables|/Game/Blueprints/BP_Player.BP_Player_C|GetStaticMesh _asbp_player) (* (Math|Vector|GetForwardVector (Variables|/Game/Blueprints/BP_Player.BP_Player_C|GetStaticMesh _asbp_player)) (Variables|Default|GetKnockBackPower)) true "None")
  (Variables|/Game/Blueprints/BP_Player.BP_Player_C|SetHealthPoints _asbp_player (- (Variables|/Game/Blueprints/BP_Player.BP_Player_C|GetHealthPoints _asbp_player) 1)))

(fn ConstructionScript)